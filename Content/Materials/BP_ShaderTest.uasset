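; BP_ShaderTest is a test Blueprint that draws a custom shader into a render target on key presses.
; BeginPlay clears ShaderTestRT to a pale color.
; Keys 1, 2 and 3 set Color to red, green or blue, then share one path into DrawTestShaderRenderTarget with WireframeTexture.
; Each draw is followed by a CallTest call.
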(event EventBeginPlay
  (Rendering|ClearRenderTarget2D "/Game/Materials/ShaderTestRT.ShaderTestRT" "(R=0.893609,G=0.942708,B=0.912537,A=1.000000)"))

(event Input|KeyboardEvents|1
  (params (Key :type Key%20Structure :default "None"))
  (:Pressed
    (Variables|Default|SetColor "(R=0.880208,G=0.078571,B=0.000000,A=1.000000)")
    (Class|TestShaderBlueprintLibrary|DrawTestShaderRenderTarget self "/Game/Materials/ShaderTestRT.ShaderTestRT" (Variables|Default|GetColor) "/Engine/EngineResources/WireframeTexture.WireframeTexture")
    (Default|CallTest)))

(event Input|KeyboardEvents|2
  (params (Key :type Key%20Structure :default "None"))
  (:Pressed
    (Variables|Default|SetColor "(R=0.023775,G=0.739583,B=0.071879,A=1.000000)")
    (Class|TestShaderBlueprintLibrary|DrawTestShaderRenderTarget self "/Game/Materials/ShaderTestRT.ShaderTestRT" (Variables|Default|GetColor) "/Engine/EngineResources/WireframeTexture.WireframeTexture")
    (Default|CallTest)))

(event Input|KeyboardEvents|3
  (params (Key :type Key%20Structure :default "None"))
  (:Pressed
    (Variables|Default|SetColor "(R=0.039298,G=0.360234,B=0.692708,A=1.000000)")
    (Class|TestShaderBlueprintLibrary|DrawTestShaderRenderTarget self "/Game/Materials/ShaderTestRT.ShaderTestRT" (Variables|Default|GetColor) "/Engine/EngineResources/WireframeTexture.WireframeTexture")
    (Default|CallTest)))

(fn ConstructionScript)